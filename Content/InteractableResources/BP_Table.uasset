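; BP_Table is an interactable customer table that requests fried rice and takes delivery from the player.
; BeginRequesting flags the table and shows a fried rice notifier.
; On Interact, a requesting table takes one fried rice from the third-person character, awards points, clears the request and hides one of the character's two carried-item meshes.
; GetInteractionType returns a fixed enum value identifying its interaction kind.
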(event `self.ReceiveBeginPlay`)

(event `/Game/InteractableResources/Interfaces/BPI_Interactable.Interact`
  (params (Interactor :type "Actor Object Reference"))
  (if (`self.isRequesting`)
    (bind _asbp_third_person_character (cast `/Game/ThirdPerson/Blueprints/BP_ThirdPersonCharacter` (`GameplayStatics.GetPlayerCharacter` 0)))
    (bind _amountfriedrice (`/Game/ThirdPerson/Blueprints/BP_ThirdPersonCharacter.AmountFriedRice` _asbp_third_person_character))
    (if (> _amountfriedrice 0)
      (set `/Game/ThirdPerson/Blueprints/BP_ThirdPersonCharacter.AmountFriedRice` (- _amountfriedrice 1) _asbp_third_person_character)
      (set `/Game/ThirdPerson/Blueprints/BP_ThirdPersonCharacter.spawnedFriedRice` (- (`/Game/ThirdPerson/Blueprints/BP_ThirdPersonCharacter.spawnedFriedRice` _asbp_third_person_character) 1) _asbp_third_person_character)
      (set `/Game/ThirdPerson/Blueprints/BP_ThirdPersonCharacter.Points` (+ (`/Game/ThirdPerson/Blueprints/BP_ThirdPersonCharacter.Points` _asbp_third_person_character) 25) _asbp_third_person_character)
      (`SceneComponent.SetVisibility` (`self.BP_FriedRiceNotifier`) false false)
      (set `self.isRequesting` false)
      (bind _staticmesh1 (`/Game/ThirdPerson/Blueprints/BP_ThirdPersonCharacter.StaticMesh1` _asbp_third_person_character))
      (if (`SceneComponent.IsVisible` _staticmesh1)
        (`SceneComponent.SetVisibility` _staticmesh1 false false)
        (else
          (`SceneComponent.SetVisibility` (`/Game/ThirdPerson/Blueprints/BP_ThirdPersonCharacter.StaticMesh` _asbp_third_person_character) false false))))
    (else
      (`KismetSystemLibrary.PrintString` "Do Nothing"))))

(event `BeginRequesting`
  (set `self.isRequesting` true)
  (`KismetSystemLibrary.PrintString` "Fried Rice Req Received")
  (`SceneComponent.SetVisibility` (`self.BP_FriedRiceNotifier`) true true))

(fn `GetInteractionType`
  (returns (type :type "/Game/InteractableResources/Interfaces/E_InteractionTypes Enum"))
  (return "NewEnumerator1"))

(fn `UserConstructionScript`)