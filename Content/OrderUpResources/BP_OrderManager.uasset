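; BP_OrderManager maintains the list of active food orders, held as Tasks and drawn at random from a recipe array.
; BeginPlay adds the first order and starts a delay timer for adding orders, which AddTask clears when it finds the list full.
; TryFinishTask completes the first order matching the submitted food name.
; FinishTask prints the name, removes the order and restarts the timer if it is no longer valid.
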(event `self.ReceiveBeginPlay`
  (`self.AddTask`)
  (`self.StartAddTimer`))

(event `StartAddTimer`
  (bind _returnvalue (`KismetSystemLibrary.K2_SetTimerDelegate` (`|CreateDelegate` :!event `AddTask`) (`self.NextTaskDelay`)))
  (set `self.AddTaskTimerHandle` _returnvalue))

(event `AddTask`
  (if (== (`KismetArrayLibrary.Array_Length` (`self.Tasks`)) (`self.MaxTasksAmmount`))
    (`KismetSystemLibrary.K2_ClearAndInvalidateTimerHandle` (`self.AddTaskTimerHandle`))
    (else
      (`KismetArrayLibrary.Array_Add` (`self.Tasks`) (`KismetArrayLibrary.Array_Random` (`self.Recipe`))))))

(event `TryFinishTask`
  (params (Ingredients :type "/Game/OrderUpResources/PDA_Order Object Reference"))
  (for (_array_element _array_index) (`self.Tasks`)
    (if (== (`/Game/OrderUpResources/PDA_Order.FoodName` _array_element) (`/Game/OrderUpResources/PDA_Order.FoodName` Ingredients))
      (`self.FinishTask` _array_index)
      (break))))

(event `FinishTask`
  (params (FinishedTaskIndex :type Integer))
  (`|ExecutionSequence`
    (:`then_0`
      (`KismetSystemLibrary.PrintString` (`/Game/OrderUpResources/PDA_Order.FoodName` (`|GetArrayItem` (`self.Tasks`) FinishedTaskIndex))))
    (:`then_1`
      (`KismetArrayLibrary.Array_Remove` (`self.Tasks`) FinishedTaskIndex)
      (if (not (`KismetSystemLibrary.K2_IsValidTimerHandle` (`self.AddTaskTimerHandle`)))
        (`self.StartAddTimer`)))))

(fn `UserConstructionScript`)